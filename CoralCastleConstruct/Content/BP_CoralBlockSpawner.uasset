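; BP_CoralBlockSpawner spawns, positions and releases coral blocks for what appears to be a block-dropping game.
; CreateBlock spawns a random class from BlockSet just below itself, stores it as the current block and passes it the FoulLine.
; MoveSpawner follows a supplied transform with a downward offset, carrying the block along, while release and readiness calls forward to that block.
; CheckHeight spawns a BP_HeightChecker below and launches its physics plane downward.
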(fn ConstructionScript)

(fn CreateBlock
  (bind _returnvalue (Transformation|GetActorTransform))
  (bind _block_set (Variables|Default|GetBlock%20Set))
  (bind _returnvalue_2 (Game|SpawnActorfromClass (Utilities|Array|Get(acopy) _block_set (Math|Random|RandomInteger (Utilities|Array|Length _block_set))) (Math|Transform|MakeTransform (- (.location _returnvalue) "0.000000,0.000000,100.000000") (.rotation _returnvalue) (.scale _returnvalue)) "Undefined" "MultiplyWithRoot" 0 0))
  (bind _asbp_coral_block (Utilities|Casting|CastToBP_CoralBlock _returnvalue_2))
  (bind _output_get (Variables|Default|SetCurrent%20Block _asbp_coral_block))
  (Variables|/Game/BP_CoralBlock.BP_CoralBlock_C|SetFoul%20Line _output_get (Variables|Default|GetFoul%20Line)))

(fn MoveSpawner
  (params (Action%20Value :type Transform))
  (bind _current_block (Variables|Default|GetCurrent%20Block))
  (Transformation|SetActorTransform (Math|Transform|MakeTransform (- (.location Action%20Value) "0.000000,0.000000,100.000000") (.rotation Action%20Value) (.scale Action%20Value)))
  (if (!= _current_block 0)
    (Default|MoveBlock _current_block (Transformation|GetActorTransform))))

(fn ReleaseBlock
  (Default|ReleaseBlock (Variables|Default|GetCurrent%20Block)))

(fn GetCurrentBlockReadiness
  (bind _readiness (Default|GetReadiness (Variables|Default|GetCurrent%20Block)))
  (return _readiness))

(fn CheckHeight
  (bind _returnvalue (Transformation|GetActorTransform))
  (bind _returnvalue_2 (Game|SpawnActorfromClass "/Game/BP_HeightChecker.BP_HeightChecker_C" (Math|Transform|MakeTransform (- (.location _returnvalue) "0.000000,0.000000,300.000000") (.rotation _returnvalue) (.scale _returnvalue)) "Undefined" "MultiplyWithRoot" 0 0))
  (bind _output_get (Variables|Default|SetHeight%20Checker _returnvalue_2))
  (Class|PrimitiveComponent|SetAllPhysicsLinearVelocity (Variables|/Game/BP_HeightChecker.BP_HeightChecker_C|GetPlane _output_get) "0.000000,0.000000,-2000.000000" false))