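; BP_HeightChecker is a probe actor that climbs vertically until it is clear of overlapping actors.
; Begin and end overlap events maintain the Overlapping list, and while it has entries each Tick stores the current Z in LastValidatedHeight, then teleports up 50 units.
; Once the list is empty it sets GotHeight, and destroys itself if ReadyToDestroy is set.
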(event Collision|EventActorEndOverlap
  (params (OtherActor :type Actor%20Object%20Reference))
  (Utilities|Array|RemoveItem (Variables|Default|GetOverlapping) OtherActor))

(event Collision|EventActorBeginOverlap
  (params (OtherActor :type Actor%20Object%20Reference))
  (Utilities|Array|Add (Variables|Default|GetOverlapping) OtherActor))

(event EventTick
  (params (DeltaSeconds :type Float%20%28single-precision%29))
  (if (Utilities|Array|IsEmpty (Variables|Default|GetOverlapping))
    (Variables|Default|SetGot%20Height true)
    (if (Variables|Default|GetReady%20To%20Destroy)
      (Actor|DestroyActor))
    (else
      (CallFunction|CheckNext))))

(fn ConstructionScript)

(fn CheckNext
  (bind _returnvalue (Transformation|GetActorLocation))
  (Variables|Default|SetLast%20Validated%20Height (.z _returnvalue))
  (Transformation|SetActorLocation (Math|Vector|MakeVector (.x _returnvalue) (.y _returnvalue) (+ (.z _returnvalue) 5e+01)) false true))