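; BP_CoralBlock is a physics block that is positioned while held, then released to fall and settle.
; MoveBlock places it 100 units below a given transform, and ReleaseBlock clears velocity and enables physics.
; A looping timer flags falls below the foul line and counts consecutive near-zero velocity checks to freeze the block and signal readiness for the next.
; It destroys itself on reset or when flagged for destruction.
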(event Custom|Velocity0Check
  (if (Variables|Default|GetReady%20To%20Destroy)
    (Actor|DestroyActor)
    (elif (< (.z (Transformation|GetWorldLocation (Variables|Default|GetStaticMesh))) (Variables|Default|GetFoul%20Line))
      (Variables|Default|SetHas%20Crossed%20Foul true)
      (elif (and (Utilities|Operators|EqualEqual (Transformation|GetComponentVelocity (Variables|Default|GetStaticMesh)) (Math|Vector|VectorZero) 0.1) (Variables|Default|GetHasBeenReleased))
        (bind _output_get (Variables|Default|SetVelocity0Counter (+ (Variables|Default|GetVelocity0Counter) 1)))
        (if (== _output_get 5)
          (Physics|SetSimulatePhysics (Variables|Default|GetStaticMesh) false)
          (Variables|Default|SetReadyForNext true))
        (else
          (Variables|Default|SetVelocity0Counter 0))))))

(event EventBeginPlay
  (Utilities|Time|SetTimerbyEvent (delegate Custom|Velocity0Check) 0.2 true))

(event EventOnReset
  (Actor|DestroyActor))

(fn ConstructionScript)

(fn ReleaseBlock
  (Variables|Default|SetHasBeenReleased true)
  (Class|PrimitiveComponent|SetAllPhysicsLinearVelocity (Variables|Default|GetStaticMesh) "0, 0, 0" false)
  (Physics|SetSimulatePhysics (Variables|Default|GetStaticMesh) true))

(fn GetReadiness
  (return (Variables|Default|GetReadyForNext)))

(fn MoveBlock
  (params (NewParam :type Transform))
  (Transformation|SetActorTransform (Math|Transform|MakeTransform (- (.location NewParam) "0.000000,0.000000,100.000000") (.rotation NewParam) (.scale NewParam))))