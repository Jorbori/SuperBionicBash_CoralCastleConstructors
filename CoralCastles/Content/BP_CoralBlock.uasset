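; BP_CoralBlock is a physics block that is positioned, released to fall, and frozen once it comes to rest.
; A looping timer destroys it when flagged, marks it fouled below the foul line, or, once released and stationary, stops physics and sets ReadyForNext.
; Tick scales the mesh up until its Z scale reaches one, and OnReset destroys the actor.
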(event Custom|Velocity0Check
  (if (Variables|Default|GetReady%20To%20Destroy)
    (Actor|DestroyActor)
    (else
      (bind _returnvalue (CallFunction|FoulCheck))
      (if _returnvalue
        (Variables|Default|SetHas%20Crossed%20Foul true)
        (else
          (bind _returnvalue_2 (CallFunction|BlockHasStopped))
          (if _returnvalue_2
            (CallFunction|FreezeBlock)))))))

(event EventBeginPlay
  (Utilities|Time|SetTimerbyEvent (delegate Custom|Velocity0Check) 0.2 true))

(event EventOnReset
  (Actor|DestroyActor))

(event EventTick
  (params (DeltaSeconds :type Float%20%28single-precision%29))
  (CallFunction|Grow))

(fn ConstructionScript)

(fn ReleaseBlock
  (Variables|Default|SetHasBeenReleased true)
  (Class|PrimitiveComponent|SetAllPhysicsLinearVelocity (Variables|Default|GetStaticMesh) "0, 0, 0" false)
  (Physics|SetSimulatePhysics (Variables|Default|GetStaticMesh) true))

(fn GetReadiness
  (return (Variables|Default|GetReadyForNext)))

(fn MoveBlock
  (params (Location :type Vector))
  (Transformation|SetActorLocation (- Location "0.000000,0.000000,500.000000") false false))

(fn FoulCheck
  (return (< (.z (Transformation|GetWorldLocation (Variables|Default|GetStaticMesh))) (Variables|Default|GetFoul%20Line))))

(fn BlockHasStopped
  (return (and (Utilities|Operators|EqualEqual (Transformation|GetComponentVelocity (Variables|Default|GetStaticMesh)) (Math|Vector|VectorZero) 0.1) (Variables|Default|GetHasBeenReleased))))

(fn FreezeBlock
  (Physics|SetSimulatePhysics (Variables|Default|GetStaticMesh) false)
  (Variables|Default|SetReadyForNext true))

(fn Grow
  (bind _staticmesh (Variables|Default|GetStaticMesh))
  (if (< (.z (Transformation|GetWorldScale (Variables|Default|GetStaticMesh))) 1.0)
    (Transformation|SetWorldScale3D _staticmesh (+ (Transformation|GetWorldScale _staticmesh) "0.200000,0.200000,0.200000"))))