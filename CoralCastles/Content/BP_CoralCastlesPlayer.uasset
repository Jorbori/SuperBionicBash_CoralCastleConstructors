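; Player pawn for the Coral Castles minigame, where the player slides sideways within bounds and drops coral blocks to build a tall stack.
; BeginPlay spawns the start island, block spawner and per-player camera controller.
; A state machine on Tick and a looping timer cycles through rising, release on any button or flex input, landing and height measurement.
; Maximum height sets the foul line and score, and fouled blocks cost points.
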(event Custom|Score/Block%20Checks
  (CallFunction|SetScore)
  (switch int (Variables|Default|GetState)
    (:2
      (CallFunction|CheckforDropCompletion))))

(event Input|EnhancedActionEvents|EnhancedInputActionIA_StrongFlex
  (params (ActionValue :type Boolean) (ElapsedSeconds :type Float%20%28double-precision%29) (TriggeredSeconds :type Float%20%28double-precision%29) (InputAction :type Input%20Action%20Object%20Reference :default "/LimbitlessBluetoothPlugin/InputActions/IA_StrongFlex.IA_StrongFlex"))
  (switch int (Variables|Default|GetState)
    (:1
      (Default|ReleaseBlock (Variables|Default|GetCoral%20Block%20Spawner))
      (Variables|Default|SetState 2))))

(event Input|EnhancedActionEvents|EnhancedInputActionIA_Button1
  (params (ActionValue :type Boolean) (ElapsedSeconds :type Float%20%28double-precision%29) (TriggeredSeconds :type Float%20%28double-precision%29) (InputAction :type Input%20Action%20Object%20Reference :default "/MinigameCore/Input/IA_Button1.IA_Button1"))
  (switch int (Variables|Default|GetState)
    (:1
      (Default|ReleaseBlock (Variables|Default|GetCoral%20Block%20Spawner))
      (Variables|Default|SetState 2))))

(event Input|EnhancedActionEvents|EnhancedInputActionIA_Button2
  (params (ActionValue :type Boolean) (ElapsedSeconds :type Float%20%28double-precision%29) (TriggeredSeconds :type Float%20%28double-precision%29) (InputAction :type Input%20Action%20Object%20Reference :default "/MinigameCore/Input/IA_Button2.IA_Button2"))
  (switch int (Variables|Default|GetState)
    (:1
      (Default|ReleaseBlock (Variables|Default|GetCoral%20Block%20Spawner))
      (Variables|Default|SetState 2))))

(event Input|EnhancedActionEvents|EnhancedInputActionIA_Button3
  (params (ActionValue :type Boolean) (ElapsedSeconds :type Float%20%28double-precision%29) (TriggeredSeconds :type Float%20%28double-precision%29) (InputAction :type Input%20Action%20Object%20Reference :default "/MinigameCore/Input/IA_Button3.IA_Button3"))
  (switch int (Variables|Default|GetState)
    (:1
      (Default|ReleaseBlock (Variables|Default|GetCoral%20Block%20Spawner))
      (Variables|Default|SetState 2))))

(event Input|EnhancedActionEvents|EnhancedInputActionIA_MediumFlex
  (params (ActionValue :type Boolean) (ElapsedSeconds :type Float%20%28double-precision%29) (TriggeredSeconds :type Float%20%28double-precision%29) (InputAction :type Input%20Action%20Object%20Reference :default "/LimbitlessBluetoothPlugin/InputActions/IA_MediumFlex.IA_MediumFlex"))
  (switch int (Variables|Default|GetState)
    (:1
      (Default|ReleaseBlock (Variables|Default|GetCoral%20Block%20Spawner))
      (Variables|Default|SetState 2))))

(event Input|EnhancedActionEvents|EnhancedInputActionIA_LightFlex
  (params (ActionValue :type Boolean) (ElapsedSeconds :type Float%20%28double-precision%29) (TriggeredSeconds :type Float%20%28double-precision%29) (InputAction :type Input%20Action%20Object%20Reference :default "/LimbitlessBluetoothPlugin/InputActions/IA_LightFlex.IA_LightFlex"))
  (switch int (Variables|Default|GetState)
    (:1
      (Default|ReleaseBlock (Variables|Default|GetCoral%20Block%20Spawner))
      (Variables|Default|SetState 2))))

(event Input|EnhancedActionEvents|EnhancedInputActionIA_Movement
  (params (ActionValue :type Vector%202D%20Structure) (ElapsedSeconds :type Float%20%28double-precision%29) (TriggeredSeconds :type Float%20%28double-precision%29) (InputAction :type Input%20Action%20Object%20Reference :default "/MinigameCore/Input/IA_Movement.IA_Movement"))
  (Class|PawnMovementComponent|AddInputVector (Variables|Default|GetFloatingPawnMovement) (Math|Vector|MakeVector 0.0 (.x ActionValue) 0.0) false)
  (CallFunction|KeepActorWtihinBound))

(event EventTick
  (params (DeltaSeconds :type Float%20%28single-precision%29))
  (CallFunction|SyncSpawner)
  (switch int (Variables|Default|GetState)
    (:0
      (CallFunction|SetUpNextBlock))
    (:3
      (CallFunction|CheckforNewMaxHeight))))

(event EventBeginPlay
  (Utilities|Time|SetTimerbyEvent (delegate Custom|Score/Block%20Checks) 0.2 true)
  (Components|Animation|PlayAnimation (Variables|Default|GetSkeletalMesh) "/BashAssets/Character/Modular/Animations/ModChara_Contemplative.ModChara_Contemplative" false)
  (CallFunction|SetCenter)
  (CallFunction|CreateStartIsland)
  (CallFunction|CreateBlockSpanwer)
  (CallFunction|CreateCameraController)
  (Default|CreateBlock (Variables|Default|GetCoral%20Block%20Spawner)))

(event EventOnReset
  (Actor|DestroyActor))

(fn ConstructionScript)

(fn SetScore
  (bind _output_get (Variables|Default|SetScore (+ (Math|Float|Truncate (Variables|Default|GetMaximum%20Height)) (Variables|Default|GetPenalty%20Points))))
  (Class|BasePointCounter|SetPoints (Class|MinigameBase|GetPointCounter (Variables|Default|GetMinigame)) (Variables|Default|GetPlayerNumber) _output_get))

(fn KeepActorWtihinBound
  (bind _returnvalue (Transformation|GetActorLocation))
  (bind _centery (Variables|Default|GetCenterY))
  (bind _returnvalue_2 (- (.y _returnvalue) _centery))
  (if (> (Math|Float|Absolute(Float) _returnvalue_2) 6e+02)
    (Transformation|SetActorLocation (Math|Vector|MakeVector (.x _returnvalue) (+ (* (Math|Float|Sign(Float) _returnvalue_2) 6e+02) (Variables|Default|GetCenterY)) (.z _returnvalue)) false false)))

(fn SetCenter
  (Variables|Default|SetCenterY (.y (Transformation|GetWorldLocation (Variables|Default|GetSkeletalMesh)))))

(fn CreateStartIsland
  (bind _returnvalue (Game|SpawnActorfromClass "/Game/BP_CoralCastlesStartIsland.BP_CoralCastlesStartIsland_C" (Math|Transform|MakeTransform (- (Transformation|GetWorldLocation (Variables|Default|GetSkeletalMesh)) "0.000000,0.000000,1600.000000") "0.000000,90.000000,0.000000" "1.000000,1.000000,1.000000") "Undefined" "MultiplyWithRoot" 0 0))
  (Variables|Default|SetStart%20Island _returnvalue))

(fn CreateBlockSpanwer
  (bind _returnvalue (Game|SpawnActorfromClass "/Game/BP_CoralBlockSpawner.BP_CoralBlockSpawner_C" (Math|Transform|MakeTransform (- (Transformation|GetWorldLocation (Variables|Default|GetSkeletalMesh)) "0.000000,0.000000,100.000000") "0, 0, 0" "1.000000,1.000000,1.000000") "Undefined" "MultiplyWithRoot" 0 0))
  (Variables|Default|SetCoral%20Block%20Spawner _returnvalue))

(fn CreateCameraController
  (bind _returnvalue (Game|SpawnActorfromClass "/Game/BP_CoralCastlesCamController.BP_CoralCastlesCamController_C" (Math|Transform|MakeTransform (- (Transformation|GetWorldLocation (Variables|Default|GetSkeletalMesh)) "2500.000000,0.000000,800.000000") "0, 0, 0" "1.000000,1.000000,1.000000") "Undefined" "MultiplyWithRoot" 0 0))
  (bind _output_get (Variables|Default|SetCamera%20Controller _returnvalue))
  (Default|AssignController _output_get (Variables|Default|GetPlayerNumber))
  (Transformation|SetActorTransform (Variables|/Game/BP_CoralCastlesCamController.BP_CoralCastlesCamController_C|GetMinigame%20Capture (Variables|Default|GetCamera%20Controller)) (Transformation|GetActorTransform (Variables|Default|GetCamera%20Controller))))

(fn MoveCamera
  (bind _returnvalue (Transformation|GetActorLocation))
  (Transformation|SetActorLocation (Variables|Default|GetCamera%20Controller) (Math|Vector|MakeVector (- (.x _returnvalue) 2.5e+03) (.y (Transformation|GetActorLocation (Variables|Default|GetCamera%20Controller))) (- (.z _returnvalue) 8e+02)) false false))

(fn CheckforNewMaxHeight
  (bind _coral_block_spawner (Variables|Default|GetCoral%20Block%20Spawner))
  (bind _height_checker (Variables|/Game/BP_CoralBlockSpawner.BP_CoralBlockSpawner_C|GetHeight%20Checker _coral_block_spawner))
  (if (Variables|/Game/BP_HeightChecker.BP_HeightChecker_C|GetGot%20Height _height_checker)
    (bind _output_get (Variables|Default|SetMaximum%20Height (Variables|/Game/BP_HeightChecker.BP_HeightChecker_C|GetLast%20Validated%20Height _height_checker)))
    (bind _output_get_2 (Variables|Default|SetFoul%20Line (- _output_get 1.5e+03)))
    (Variables|/Game/BP_CoralBlockSpawner.BP_CoralBlockSpawner_C|SetFoul%20Line (Variables|Default|GetCoral%20Block%20Spawner) _output_get_2)
    (Variables|Default|SetState 0)
    (Variables|/Game/BP_HeightChecker.BP_HeightChecker_C|SetReady%20To%20Destroy (Variables|/Game/BP_CoralBlockSpawner.BP_CoralBlockSpawner_C|GetHeight%20Checker (Variables|Default|GetCoral%20Block%20Spawner)) true)))

(fn CheckforDropCompletion
  (bind _coral_block_spawner (Variables|Default|GetCoral%20Block%20Spawner))
  (bind _readiness (Default|GetCurrentBlockReadiness _coral_block_spawner))
  (if _readiness
    (Variables|Default|SetState 3)
    (Default|SpawnHeightChecker (Variables|Default|GetCoral%20Block%20Spawner) (Variables|Default|GetCenterY) (Variables|Default|GetMaximum%20Height))
    (Default|CreateBlock (Variables|Default|GetCoral%20Block%20Spawner) :!label _label)
    (elif (Variables|/Game/BP_CoralBlock.BP_CoralBlock_C|GetHas%20Crossed%20Foul (Variables|/Game/BP_CoralBlockSpawner.BP_CoralBlockSpawner_C|GetCurrent%20Block _coral_block_spawner))
      (Variables|/Game/BP_CoralBlock.BP_CoralBlock_C|SetReady%20To%20Destroy (Variables|/Game/BP_CoralBlockSpawner.BP_CoralBlockSpawner_C|GetCurrent%20Block _coral_block_spawner) true)
      (Variables|Default|SetState 0)
      (Variables|Default|SetPenalty%20Points (- (Variables|Default|GetPenalty%20Points) 150))
      (goto _label))))

(fn SetUpNextBlock
  (bind _returnvalue (CallFunction|IsSpawneratCorrectHeight))
  (if _returnvalue
    (Variables|Default|SetState 1)
    (else
      (Class|PawnMovementComponent|AddInputVector (Variables|Default|GetFloatingPawnMovement) (Math|Vector|MakeVector 0.0 0.0 1.0) false)
      (Default|MoveSpawner (Variables|Default|GetCoral%20Block%20Spawner) (Transformation|GetActorLocation))
      (CallFunction|MoveCamera))))

(fn SyncSpawner
  (Default|MoveSpawner (Variables|Default|GetCoral%20Block%20Spawner) (Transformation|GetWorldLocation (Variables|Default|GetSkeletalMesh))))

(fn IsSpawneratCorrectHeight
  (return (>= (.z (.location (Transformation|GetBoneTransform (Variables|Default|GetSkeletalMesh) "None" "RTS_World"))) (+ 1.5e+03 (Variables|Default|GetMaximum%20Height)))))