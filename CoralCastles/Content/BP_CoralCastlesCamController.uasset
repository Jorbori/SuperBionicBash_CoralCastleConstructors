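; BP_CoralCastlesCamController drives a minigame capture actor, apparently as the camera for the Coral Castles minigame.
; AssignController finds the BP_MinigameCapture whose capture number matches the one passed in and stores it.
; Every tick it copies its own transform onto that capture, so the capture follows this actor.
; It destroys itself on reset.
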(event EventTick
  (params (DeltaSeconds :type Float%20%28single-precision%29))
  (Transformation|SetActorTransform (Variables|Default|GetMinigame%20Capture) (Transformation|GetActorTransform)))

(event EventOnReset
  (Actor|DestroyActor))

(fn ConstructionScript)

(fn AssignController
  (params (Capture%20Number :type Integer))
  (bind _outactors (Actor|GetAllActorsOfClass "/MinigameCore/Game/BP_MinigameCapture.BP_MinigameCapture_C"))
  (for _array_element _outactors
    (if (== (Class|MinigameCapture|GetCaptureNumber _array_element) Capture%20Number)
      (bind _output_get (Variables|Default|SetMinigame%20Capture _array_element)))))